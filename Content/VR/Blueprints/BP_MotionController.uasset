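; VR hand actor that picks up and drops interactable objects, serving either hand by mirroring one hand mesh for the left.
; Pickup finds the nearest BPI_Interactable actor overlapping GrabSphere and messages it with the hand mesh.
; Drop messages the object only if still attached to this hand, allowing for hand-to-hand transfers.
; Tick derives a grip state from nearby objects and grab status, feeding it to RightHand_AnimBP.
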(event `self.ReceiveBeginPlay`
  (switch `EControllerHand` (`self.Hand`)
    (:`Left`
      (`SceneComponent.SetWorldScale3D` (`self.HandMesh`) (1.0 1.0 -1.0)))))

(event `PickUpItem`
  (bind _nearestactor (`self.FindNearestObject`))
  (`/Engine/EditorBlueprintResources/StandardMacros.IsValid` _nearestactor
    (:`Is Valid`
      (set `self.GrabbingObject` _nearestactor)
      (set `self.bGrabbing` true)
      (message `/Game/VR/Blueprints/BPI_Interactable.PickUp` _nearestactor (`self.HandMesh`)))))

(event `DropItem`
  (bind _grabbingobject (`self.GrabbingObject`))
  (`/Engine/EditorBlueprintResources/StandardMacros.IsValid` _grabbingobject
    (:`Is Valid`
      (set `self.bGrabbing` false)
      (if (== (`SceneComponent.GetAttachParent` (`Actor.RootComponent` _grabbingobject)) (`self.HandMesh`))
        (message `/Game/VR/Blueprints/BPI_Interactable.Drop` _grabbingobject)
        (else
          (set `self.GrabbingObject` null))))))

(event `self.ReceiveTick`
  (params (DeltaSeconds :type "Float (single-precision)"))
  (`|ExecutionSequence`
    (:`then_0`
      (bind _nearestactor (`self.FindNearestObject`))
      (`/Engine/EditorBlueprintResources/StandardMacros.IsValid` _nearestactor
        (:`Is Valid`
          (if (`self.bGrabbing`)
            (set `self.GripState` "NewEnumerator2")
            (else
              (set `self.GripState` "NewEnumerator1"))))
        (:`Is Not Valid`
          (set `self.GripState` "NewEnumerator0"))))
    (:`then_1`
      (bind _asright_hand_anim_bp (cast `/Game/VirtualReality/Mannequin/Animations/RightHand_AnimBP` (`SkeletalMeshComponent.GetAnimInstance` (`self.HandMesh`))))
      (set `/Game/VirtualReality/Mannequin/Animations/RightHand_AnimBP.GripState` (`self.GripState`) _asright_hand_anim_bp))))

(fn `FindNearestObject`
  (returns (NearestActor :type "Actor Object Reference"))
  (locals (NearestDistance :type "Float (double-precision)") (TestObject :type "Actor Object Reference") (NearestObject :type "Actor Object Reference"))
  (bind _returnvalue (`KismetMathLibrary.VSize` (- (`self.K2_GetActorLocation` (`local.TestObject`)) (`SceneComponent.K2_GetComponentLocation` (`self.GrabSphere`)))))
  (set `local.NearestDistance` 10000.0)
  (for _array_element (`PrimitiveComponent.GetOverlappingActors` (`self.GrabSphere`) "/Script/Engine.Actor")
    (bind _output_get (set `local.TestObject` _array_element))
    (if (`KismetSystemLibrary.DoesImplementInterface` _output_get "/Game/VR/Blueprints/BPI_Interactable.BPI_Interactable_C")
      (if (< _returnvalue (`local.NearestDistance`))
        (set `local.NearestDistance` _returnvalue)
        (set `local.NearestObject` (`local.TestObject`)))))
  (return (`local.NearestObject`)))

(fn `UserConstructionScript`
  (set `MotionControllerComponent.Hand` (`self.Hand`) (`self.MotionController`)))