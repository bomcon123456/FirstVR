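; BP_RayActor is a VR actor that gives visual feedback to trace interaction callbacks, apparently as a test or example target.
; Its Cube changes its Color material parameter: red on hover, green while activated, red on release and white when the trace leaves.
; TraceMoveTick places the Arrow at the hit point, oriented along the surface normal.
; Component enter and leave callbacks are empty, and every callback returns false.
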(fn `TraceActiveDown`
  (params (Hit :type "HitResult Structure") (Instigator :type "Pawn Object Reference"))
  (returns (Return :type Boolean))
  (`MeshComponent.SetVectorParameterValueOnMaterials` (`self.Cube`) "Color" (0.0 1.0 0.0))
  (return false))

(fn `TraceActiveUp`
  (params (Hit :type "HitResult Structure") (Instigator :type "Pawn Object Reference"))
  (returns (Return :type Boolean))
  (`MeshComponent.SetVectorParameterValueOnMaterials` (`self.Cube`) "Color" (1.0 0.0 0.0))
  (return false))

(fn `TraceHitComponent`
  (params (Hit :type "HitResult Structure") (HitComponent :type "PrimitiveComponent Object Reference"))
  (returns (Return :type Boolean))
  (return false))

(fn `TraceHitObject`
  (params (Hit :type "HitResult Structure"))
  (returns (Return :type Boolean))
  (`MeshComponent.SetVectorParameterValueOnMaterials` (`self.Cube`) "Color" (1.0 0.0 0.0))
  (return false))

(fn `TraceLeaveComponent`
  (params (Hit :type "HitResult Structure") (HitComponent :type "PrimitiveComponent Object Reference"))
  (returns (Return :type Boolean))
  (return false))

(fn `TraceLeaveObject`
  (params (Hit :type "HitResult Structure"))
  (returns (Return :type Boolean))
  (`MeshComponent.SetVectorParameterValueOnMaterials` (`self.Cube`) "Color" (1.0 1.0 1.0))
  (return false))

(fn `TraceMoveTick`
  (params (Hit :type "HitResult Structure (by ref)"))
  (returns (Return :type Boolean))
  (`SceneComponent.K2_SetWorldLocationAndRotation` (`self.Arrow`) Hit_Location (`KismetMathLibrary.MakeRotFromX` Hit_Normal) false false)
  (return false))

(fn `UserConstructionScript`)