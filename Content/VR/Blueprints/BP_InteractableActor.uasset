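; BP_InteractableActor is a VR actor with a static mesh that can be picked up, dropped and targeted by traces.
; PickUp disables physics and attaches the mesh to the given component, keeping its world transform; Drop re-enables physics and detaches it.
; TraceHitObject tints the mesh red through its Color material parameter, and nothing reverts it.
; The other trace callbacks are empty or return false.
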(event `/Game/VR/Blueprints/BPI_Interactable.PickUp`
  (params (AttachTo :type "SceneComponent Object Reference"))
  (bind _staticmesh (`self.StaticMesh`))
  (`PrimitiveComponent.SetSimulatePhysics` _staticmesh false)
  (`SceneComponent.K2_AttachToComponent` _staticmesh AttachTo "None" "KeepWorld" "KeepWorld" "KeepWorld" false))

(event `/Game/VR/Blueprints/BPI_Interactable.Drop`
  (`PrimitiveComponent.SetSimulatePhysics` (`self.StaticMesh`) true)
  (`SceneComponent.K2_DetachFromComponent` (`self.StaticMesh`) "KeepWorld" "KeepWorld" "KeepWorld" true))

(fn `TraceActiveDown`
  (params (Hit :type "HitResult Structure") (Instigator :type "Pawn Object Reference"))
  (returns (Return :type Boolean))
  (return false))

(fn `TraceActiveUp`
  (params (Hit :type "HitResult Structure") (Instigator :type "Pawn Object Reference"))
  (returns (Return :type Boolean))
  (return false))

(fn `TraceHitComponent`
  (params (Hit :type "HitResult Structure") (HitComponent :type "PrimitiveComponent Object Reference"))
  (returns (Return :type Boolean))
  (return false))

(fn `TraceHitObject`
  (params (Hit :type "HitResult Structure"))
  (returns (Return :type Boolean))
  (`MeshComponent.SetVectorParameterValueOnMaterials` (`self.StaticMesh`) "Color" (1.0 0.0 0.0))
  (return false))

(fn `TraceLeaveComponent`
  (params (Hit :type "HitResult Structure") (HitComponent :type "PrimitiveComponent Object Reference"))
  (returns (Return :type Boolean))
  (return false))

(fn `TraceLeaveObject`
  (params (Hit :type "HitResult Structure"))
  (returns (Return :type Boolean)))

(fn `TraceMoveTick`
  (params (Hit :type "HitResult Structure (by ref)"))
  (returns (Return :type Boolean))
  (return false))

(fn `UserConstructionScript`)