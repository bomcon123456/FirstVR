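; VR interaction component that casts a gated per-tick parabolic trace, noted as for teleport, from its own transform to drive focus on BPI_RayCast actors.
; The arc chains gravity-adjusted line traces until one hits.
; InteractWithHit tracks the focused actor and component, sending hit, leave and move-tick interface messages, while ActivateUp/Down forward to the focused actor.
; An eye line trace is disconnected, and a closest-object search has no caller here.
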(event `self.ReceiveTick`
  (params (DeltaSeconds :type "Float (single-precision)"))
  (`/Engine/EditorBlueprintResources/StandardMacros.Gate` false :!label _label
    (:`Exit`
      (bind _hit (`self.ParabolicTrace` 10 0.1 1000.0)) ; for teleport
      (bind _output_get (set `self.FocusHit` _hit))
      (`self.InteractWithHit` _output_get))))

(event `Enable`
  (goto _label :!via `Open`))

(event `Disable`
  (goto _label :!via `Close`))

(event `ActivateUp`
  (params (Instigator :type "Pawn Object Reference"))
  ;[1 1 1] Call Trace ActiveUp/Down in FocusObject
  (message `/Game/VR/Blueprints/BPI_RayCast.TraceActiveUp` (`self.FocusObject`) (`self.FocusHit`) Instigator))

(event `ActivateDown`
  (params (Instigator :type "Pawn Object Reference"))
  ;[1 1 1] Call Trace ActiveUp/Down in FocusObject
  (message `/Game/VR/Blueprints/BPI_RayCast.TraceActiveDown` (`self.FocusObject`) (`self.FocusHit`) Instigator))

(fn `InteractWithHit`
  (params (Hit :type "HitResult Structure"))
  (locals (CurrentObject :type "Actor Object Reference") (CurrentComponent :type "PrimitiveComponent Object Reference") (CurrentHit :type "HitResult Structure") (LowestArcDistance :type "Float (double-precision)" :default 0.0) (LowestVectorDistance :type "Float (double-precision)" :default 0.0) (TempObj :type "Actor Object Reference"))
  (bind _currentobject (`local.CurrentObject`))
  ;[1 1 1] Setting Up Variable
  (bind _output_get (set `local.CurrentHit` Hit))
  (`/Engine/EditorBlueprintResources/StandardMacros.IsValid` (`.HitActor` (`GameplayStatics.BreakHitResult` _output_get))
    (:`Is Valid`
      (set `local.CurrentObject` (`.HitActor` (`GameplayStatics.BreakHitResult` _output_get)))
      (set `local.CurrentComponent` (`.HitComponent` (`GameplayStatics.BreakHitResult` _output_get)))
      ;[1 1 1] Same Object (FocusObject)
      (if (== (`self.FocusObject`) (`local.CurrentObject`))
        (message `/Game/VR/Blueprints/BPI_RayCast.TraceMoveTick` (`self.FocusObject`) (`local.CurrentHit`)) ; If yes, doing something (Implement TraceMoveTick)
        (if (not (== (`self.FocusComponent`) (`local.CurrentComponent`)))
          ;[1 1 1] Sth happen with the old component/ then Hit new Comp + set new Comp to FocusComp
          (message `/Game/VR/Blueprints/BPI_RayCast.TraceLeaveComponent` (`self.FocusObject`) (`local.CurrentHit`) (`self.FocusComponent`))
          (message `/Game/VR/Blueprints/BPI_RayCast.TraceHitComponent` (`self.FocusObject`) (`local.CurrentHit`) (`local.CurrentComponent`))
          (set `self.FocusComponent` (`local.CurrentComponent`)))
        (else
          ;[1 1 1] Leave FocusedObject
          (message `/Game/VR/Blueprints/BPI_RayCast.TraceLeaveObject` (`self.FocusObject`) (`local.CurrentHit`))
          (set `self.FocusObject` null)
          (set `self.FocusComponent` null)
          (if (`KismetSystemLibrary.DoesImplementInterface` _currentobject "/Game/VR/Blueprints/BPI_RayCast.BPI_RayCast_C")
            ;[1 1 1] Hit new object/compo
            (message `/Game/VR/Blueprints/BPI_RayCast.TraceHitObject` _currentobject (`local.CurrentHit`))
            (message `/Game/VR/Blueprints/BPI_RayCast.TraceHitComponent` (`local.CurrentObject`) (`local.CurrentHit`) (`local.CurrentComponent`))
            (set `self.FocusObject` (`local.CurrentObject`))
            (set `self.FocusComponent` (`local.CurrentComponent`))))))))

(fn `LineTrace`
  (params (Distance :type "Float (double-precision)"))
  (returns (Hit :type "HitResult Structure"))
  (bind _returnvalue (`GameplayStatics.GetPlayerCameraManager` 0))
  (bind _returnvalue_2 (`PlayerCameraManager.GetCameraLocation` _returnvalue))
  (bind _outhit (`KismetSystemLibrary.LineTraceSingle` :`Start` _returnvalue_2 :`End` (+ _returnvalue_2 (* (`Actor.GetActorForwardVector` _returnvalue) Distance)) :`TraceChannel` "TraceTypeQuery1" :`DrawDebugType` "ForOneFrame" :`TraceColor` (struct :`G` 1.0 :`B` 0.9024 :`A` 1.0) :`DrawTime` 2.0))
  (return _outhit))

(fn `ParabolicTrace`
  (params (Steps :type Integer) (StepLength :type "Float (double-precision)") (Speed :type "Float (double-precision)"))
  (returns (Hit :type "HitResult Structure"))
  (locals (InitialPosition :type "Vector Structure") (PreviousPosition :type "Vector Structure") (Velocity :type "Vector Structure") (inSteps :type Integer) (inStepLength :type "Float (double-precision)") (inHit :type "HitResult Structure"))
  (bind (_velocity_x _velocity_y _velocity_z) (`KismetMathLibrary.BreakVector` (`local.Velocity`)))
  ;[1 1 1] Initial Setup
  (set `local.inSteps` Steps)
  (set `local.inStepLength` StepLength)
  (set `local.Velocity` (* (`self.GetForwardVector`) Speed))
  (bind _output_get (set `local.InitialPosition` (`self.K2_GetComponentLocation`)))
  (set `local.PreviousPosition` _output_get)
  (for _index (range 1 (+ (`local.inSteps`) 1))
    (bind _returnvalue (* _index (`local.inStepLength`)))
    (bind _returnvalue_2 (+ (`KismetMathLibrary.MakeVector` (* _returnvalue _velocity_x) (* _returnvalue _velocity_y) (- (* _returnvalue _velocity_z) (* _returnvalue _returnvalue 980.0 0.5))) (`local.InitialPosition`)))
    (bind (_outhit _returnvalue_3) (`KismetSystemLibrary.LineTraceSingle` :`Start` (`local.PreviousPosition`) :`End` _returnvalue_2 :`TraceChannel` "TraceTypeQuery1" :`DrawDebugType` "ForOneFrame" :`TraceColor` (struct :`R` 0.822917 :`G` 0.269903 :`B` 0.444993 :`A` 1.0)))
    (set `local.PreviousPosition` _returnvalue_2)
    (set `local.inHit` _outhit)
    (if _returnvalue_3
      (break)))
  (return (`local.inHit`)))

(fn `TraceActiveDown`
  (params (Hit :type "HitResult Structure") (Instigator :type "Pawn Object Reference"))
  (returns (Return :type Boolean))
  (return false))

(fn `TraceActiveUp`
  (params (Hit :type "HitResult Structure") (Instigator :type "Pawn Object Reference"))
  (returns (Return :type Boolean))
  (return false))

(fn `TraceHitComponent`
  (params (Hit :type "HitResult Structure") (HitComponent :type "PrimitiveComponent Object Reference"))
  (returns (Return :type Boolean))
  (return false))

(fn `TraceHitObject`
  (params (Hit :type "HitResult Structure"))
  (returns (Return :type Boolean))
  (return false))

(fn `TraceLeaveComponent`
  (params (Hit :type "HitResult Structure") (HitComponent :type "PrimitiveComponent Object Reference"))
  (returns (Return :type Boolean))
  (return false))

(fn `TraceLeaveObject`
  (params (Hit :type "HitResult Structure"))
  (returns (Return :type Boolean))
  (return false))

(fn `TraceMoveTick`
  (params (Hit :type "HitResult Structure (by ref)"))
  (returns (Return :type Boolean))
  (return false))